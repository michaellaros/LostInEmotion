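; Game instance that manages the main and multiplayer menus, solo game launch, multiplayer sessions and the player profile.
; It creates or joins LAN or online sessions, hosts the lobby as a listen server and uses servertravel to change maps.
; Showing the main menu loads or creates the SG_PlayerProfile save to fill the name field.
; SaveProfile writes only when its cached save object is invalid, so later name changes are not saved.
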(event `StartSoloGame`
  (set `self.IsSoloGame` true)
  (`GameplayStatics.OpenLevel` "ThirdPersonMap"))

(event `ChangePlayerName`
  (params (PlayerName :type Text))
  (set `self.Player Profile_Info` (make `/Game/SavedData/S_PlayerProfile` PlayerName))
  (`self.SaveProfile`))

(event `CreateMPSession`
  (set `self.IsSoloGame` false)
  (`CreateSessionCallbackProxy.CreateSession` (`GameplayStatics.GetPlayerController` 0) 4 (`self.IsLanConnection`)
    (:`OnSuccess`
      (`GameplayStatics.OpenLevel` "LobbyMenu_Map" true "listen"))
    (:`OnFailure`
      (`KismetSystemLibrary.PrintString` "Failed to create session"))))

(event `JoinMPSession`
  (params (SearchResult :type "BlueprintSessionResult Structure (by ref)"))
  (set `self.IsSoloGame` false)
  (`JoinSessionCallbackProxy.JoinSession` (`GameplayStatics.GetPlayerController` 0) SearchResult
    (:`OnFailure`
      (`KismetSystemLibrary.PrintString` "Failed toJoin session"))))

(event `TravelToMap`
  (params (ConnectedPlayers :type Integer) (MapName :type String))
  (set `self.ConnectedPlayers` ConnectedPlayers)
  (`KismetSystemLibrary.ExecuteConsoleCommand` (`KismetStringLibrary.Concat_StrStr` "servertravel " MapName) (`GameplayStatics.GetPlayerController` 0)))

(fn `ChangeConnectionType`
  (returns (IsLanConnection :type Boolean))
  (if (`self.IsLanConnection`)
    (set `self.IsLanConnection` false)
    (return (`self.IsLanConnection`))
    (else
      (set `self.IsLanConnection` true))))

(fn `CheckForSaveProfile`
  (bind _returnvalue (`GameplayStatics.DoesSaveGameExist` (`self.PlayerProfileSlot`)))
  (if _returnvalue
    (`self.LoadProfile`)
    (else
      (`self.SaveProfile`)))
  (return))

(fn `LoadProfile`
  (bind _returnvalue (`GameplayStatics.LoadGameFromSlot` (`self.PlayerProfileSlot`)))
  (bind _assg_player_profile (cast `/Game/SavedData/SG_PlayerProfile` _returnvalue))
  (set `self.Player Profile_Info` (`/Game/SavedData/SG_PlayerProfile.PlayerProfile` _assg_player_profile))
  (return))

(fn `SaveProfile`
  (bind _sg_playerprofile (`self.SG_PlayerProfile`))
  (`/Engine/EditorBlueprintResources/StandardMacros.IsValid` (`self.SG_PlayerProfile`)
    (:`Is Not Valid`
      (bind _returnvalue (`GameplayStatics.CreateSaveGameObject` "/Game/SavedData/SG_PlayerProfile.SG_PlayerProfile_C"))
      (set `self.SG_PlayerProfile` _returnvalue)
      (set `/Game/SavedData/SG_PlayerProfile.PlayerProfile` (`self.Player Profile_Info`) _sg_playerprofile)
      (`GameplayStatics.SaveGameToSlot` _sg_playerprofile (`self.PlayerProfileSlot`))
      (return))))

(fn `UI_ShowMainMenu`
  (bind _returnvalue (`GameplayStatics.GetPlayerController` 0))
  (`/Engine/EditorBlueprintResources/StandardMacros.IsValid` (`self.WB_MainMenu`)
    (:`Is Valid`
      _)
    (:`Is Not Valid`
      (bind _returnvalue_2 (`|CreateWidget` "/Game/UI/WB_MainMenu.WB_MainMenu_C" _returnvalue))
      (set `self.WB_MainMenu` _returnvalue_2)))
  (`UserWidget.AddToViewport` (`self.WB_MainMenu`) 0)
  (`WidgetBlueprintLibrary.SetInputMode_UIOnlyEx` _returnvalue null)
  (set `PlayerController.bShowMouseCursor` true _returnvalue)
  (`self.CheckForSaveProfile`)
  (`EditableText.SetText` (`/Game/UI/WB_MainMenu.InputPlayerName` (`self.WB_MainMenu`)) (`.PlayerName_2_718E7E1347427B6EE20F71AB236F4B4A` (break `/Game/SavedData/S_PlayerProfile` (`self.Player Profile_Info`))))
  (return))

(fn `UI_ShowMpMenu`
  (`/Engine/EditorBlueprintResources/StandardMacros.IsValid` (`self.WB_MpMenu`)
    (:`Is Valid`
      _)
    (:`Is Not Valid`
      (bind _returnvalue (`|CreateWidget` "/Game/UI/WB_MpMainMenu.WB_MpMainMenu_C" (`GameplayStatics.GetPlayerController` 0)))
      (set `self.WB_MpMenu` _returnvalue)))
  (`UserWidget.AddToViewport` (`self.WB_MpMenu`) 0)
  (return))