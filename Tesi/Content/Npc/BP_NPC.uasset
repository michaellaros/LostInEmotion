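; NPC character that follows the first player's BP_ThirdPersonCharacter_P1 once interacted with, until it reaches an ArrivePoint.
; Interact starts a self-calling FollowPlayer loop on a short delay, using AIMoveTo toward the player, or toward itself when already close.
; Overlapping an ArrivePoint clears the follow flag, so the next loop pass halts movement.
; Separate events switch between run and walk speeds; Change is an empty stub.
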(event `self.ReceiveBeginPlay`
  (bind _asbp_third_person_character_p1 (cast `/Game/ThirdPerson/Blueprints/BP_ThirdPersonCharacter_P1` (`GameplayStatics.GetPlayerCharacter` 0)))
  (set `self.As BP Third Person Character P1` _asbp_third_person_character_p1))

(event `FollowPlayer`
  (bind _as_bp_third_person_character_p1 (`self.As BP Third Person Character P1`))
  (if (`self.FollowPlayer?`)
    (if (>= (`self.GetDistanceTo` _as_bp_third_person_character_p1) 200.0)
      (`|AIMoveTo` self (0.0 0.0 0.0) _as_bp_third_person_character_p1
        (:`then`
          _))
      (else
        (`|AIMoveTo` self (0.0 0.0 0.0) self
          (:`then`
            _))))
    (`KismetSystemLibrary.Delay` 0.2)
    (`self.FollowPlayer`)
    (else
      (`MovementComponent.StopMovementImmediately` (`self.CharacterMovement`)))))

(event `self.ReceiveActorBeginOverlap`
  (params (OtherActor :type "Actor Object Reference"))
  (cast `/Game/Npc/ArrivePoint` OtherActor)
  (set `self.FollowPlayer?` false))

(event `SetRunSpeed`
  (set `CharacterMovementComponent.MaxWalkSpeed` 1100.0 (`self.CharacterMovement`)))

(event `SetWalkSpeed`
  (set `CharacterMovementComponent.MaxWalkSpeed` 550.0 (`self.CharacterMovement`)))

(fn `Change`)

(fn `Interact`
  (params (Interactor :type "Character Object Reference"))
  (returns (`Success?` :type Boolean))
  (`self.FollowPlayer`)
  (return false))

(fn `UserConstructionScript`)