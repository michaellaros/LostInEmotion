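; Player 2's NPC that receives the first P2 collectible when the player interacts with it to deliver the item.
; The construction script applies the AliasMaster material to its mesh.
; Interact requires the P2 character and checks the game mode's IsCollected1P2 flag.
; If set, it spawns a display copy of the collectible, disables its collision, attaches it to the mesh's CollectibleSocket and calls GiveCollectible on the character.
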(fn `Interact`
  (params (Interactor :type "Character Object Reference"))
  (returns (`Success?` :type Boolean))
  ;[1 1 1] consegna dell'oggetto all'npc
  (bind _asbp_third_person_character_p2 (cast `/Game/ThirdPerson/Blueprints/BP_ThirdPersonCharacter_P2` Interactor))
  (bind _asbp_third_person_game_mode (cast `/Game/ThirdPerson/Blueprints/BP_ThirdPersonGameMode` (`GameplayStatics.GetGameMode`)))
  (if (`/Game/ThirdPerson/Blueprints/BP_ThirdPersonGameMode.isCollected1P2` _asbp_third_person_game_mode)
    (bind _returnvalue (`|SpawnActorFromClass` "/Game/Collectibles/P2/BP_Collectible1_P2.BP_Collectible1_P2_C" (`SceneComponent.GetSocketTransform` (`self.Mesh`) "CollectibleSocket" "RTS_World") "Undefined" "OverrideRootScale" null null))
    (bind _output_get (set `self.NewVar_0` _returnvalue))
    (`PrimitiveComponent.SetCollisionEnabled` (`/Game/Collectibles/P2/BP_Collectible1_P2.Box` _output_get) "NoCollision")
    (`PrimitiveComponent.SetCollisionEnabled` (`/Game/Collectibles/P2/BP_Collectible1_P2.Cube` _output_get) "NoCollision")
    (`self.K2_AttachToComponent` _output_get (`self.Mesh`) "CollectibleSocket" "SnapToTarget" "SnapToTarget" "SnapToTarget" true)
    (`/Game/ThirdPerson/Blueprints/BP_ThirdPersonCharacter_P2.GiveCollectible` _asbp_third_person_character_p2)
    (return false)))

(fn `UserConstructionScript`
  (`PrimitiveComponent.SetMaterial` (`self.Mesh`) 0 "/DatasmithContent/Materials/AliasMaster.AliasMaster"))